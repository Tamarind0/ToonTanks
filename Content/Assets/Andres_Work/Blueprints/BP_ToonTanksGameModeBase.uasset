(event EventLevelOver
  (params (bWonGame :type Boolean))
  (bind _returnvalue (Game|GetCurrentLevelName true))
  (switch string _returnvalue
    (:Default
      (bind _returnvalue_2 (UserInterface|CreateWidget "/Game/Assets/Andres_Work/Blueprints/Widgets/WBP_Level3End.WBP_Level3End_C"))
      (UserInterface|Viewport|AddtoViewport _returnvalue_2 0)
      (Variables|/Script/Engine.PlayerController|SetbShowMouseCursor (Game|GetPlayerController 0) true))
    (:Level1
      (bind _returnvalue_3 (UserInterface|CreateWidget "/Game/Assets/Andres_Work/Blueprints/Widgets/WBP_Level1End.WBP_Level1End_C"))
      (UserInterface|Viewport|AddtoViewport _returnvalue_3 0)
      (Variables|/Script/Engine.PlayerController|SetbShowMouseCursor (Game|GetPlayerController 0) true))
    (:Level2
      (bind _returnvalue_4 (UserInterface|CreateWidget "/Game/Assets/Andres_Work/Blueprints/Widgets/WBP_Level2End.WBP_Level2End_C"))
      (UserInterface|Viewport|AddtoViewport _returnvalue_4 0)
      (Variables|/Script/Engine.PlayerController|SetbShowMouseCursor (Game|GetPlayerController 0) true))))

(event EventStartGame
  (bind _returnvalue (Game|GetCurrentLevelName true))
  (switch string _returnvalue
    (:Default
      (bind _returnvalue_2 (UserInterface|CreateWidget "/Game/Assets/Andres_Work/Blueprints/Widgets/WBP_StartGameWidget.WBP_StartGameWidget_C"))
      (UserInterface|Viewport|AddtoViewport _returnvalue_2 0))))

(event EventGameOver
  (params (bWonGame :type Boolean))
  (bind _returnvalue (UserInterface|CreateWidget "/Game/Assets/Andres_Work/Blueprints/Widgets/WBP_EndGameWidget.WBP_EndGameWidget_C"))
  (UserInterface|Viewport|AddtoViewport _returnvalue 0)
  (Rendering|Components|TextRender|SetText (Variables|/Game/Assets/Andres_Work/Blueprints/Widgets/WBP_EndGameWidget.WBP_EndGameWidget_C|GetDisplayText _returnvalue) (select bWonGame "" "You Died!"))
  (Variables|/Script/Engine.PlayerController|SetbShowMouseCursor (Game|GetPlayerController 0) true))

(fn ConstructionScript)